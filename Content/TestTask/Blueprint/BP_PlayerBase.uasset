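; Base player character for a networked shooter with movement, weapon switching, firing, reloading and aiming; input starts disabled.
; Fire, reload, weapon swap, aim-offset rotation and death go through server-to-multicast events, with death disabling input and ragdolling the mesh.
; WeaponComponent supplies the current gun and triggers socket attachment and fire montages, while HealthComponent triggers death.
; Local aiming uses a timeline to blend spring arm length and camera FOV.
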(event `InputAxis|MoveForward`
  (params (AxisValue :type "Float (single-precision)"))
  ;[0.099 0.219 0.36 1 32] Игрок
  ;;[0.02604 0.02604 0.02604 1 24] Скрипты
  (`self.AddMovementInput` (`self.GetActorForwardVector`) AxisValue))

(event `InputAxis|Turn`
  (params (AxisValue :type "Float (single-precision)"))
  ;[0.099 0.219 0.36 1 32] Игрок
  ;;[0.02604 0.02604 0.02604 1 24] Скрипты
  (`self.AddControllerYawInput` AxisValue))

(event `InputAxis|LookUp`
  (params (AxisValue :type "Float (single-precision)"))
  ;[0.099 0.219 0.36 1 32] Игрок
  ;;[0.02604 0.02604 0.02604 1 24] Скрипты
  (`self.AddControllerPitchInput` AxisValue)
  (`self.ROS_UpdateOffset`))

(event `InputAxis|MoveRight`
  (params (AxisValue :type "Float (single-precision)"))
  ;[0.099 0.219 0.36 1 32] Игрок
  ;;[0.02604 0.02604 0.02604 1 24] Скрипты
  (`self.AddMovementInput` (`self.GetActorRightVector`) AxisValue))

(event `ROS_UpdateOffset`
  ;[0.099 0.219 0.36 1 32] Игрок
  ;;[0.02604 0.02604 0.02604 1 24] Скрипты
  (`self.MC_UpdateOffset`))

(event `MC_UpdateOffset`
  ;[0.099 0.219 0.36 1 32] Игрок
  ;;[0.02604 0.02604 0.02604 1 24] Скрипты
  (if (or (`self.HasAuthority`) (`self.IsLocallyControlled`))
    (set `self.Controll Rotation Rep` (`Controller.GetControlRotation` (`self.GetController`)))))

(event `InputAction|Fire` :paused true
  (params (Key :type "Key Structure"))
  ;[0.099 0.219 0.36 1 32] Игрок
  ;;[0.02604 0.02604 0.02604 1 24] Скрипты
  (:`Pressed`
    (`self.ROS_SetFire` true))
  (:`Released`
    (`self.ROS_SetFire` false)))

(event `InputAction|Reload`
  (params (Key :type "Key Structure"))
  ;[0.099 0.219 0.36 1 32] Игрок
  ;;[0.02604 0.02604 0.02604 1 24] Скрипты
  (:`Pressed`
    (`self.ROS_OnReload`)))

(event `ROS_SetGunSelect`
  (params (NewHolster :type "EHolster Enum" :default "EH_None"))
  ;[0.099 0.219 0.36 1 32] Игрок
  ;;[0.02604 0.02604 0.02604 1 24] Скрипты
  (`self.MC_SetGunSelect` NewHolster))

(event `MC_SetGunSelect`
  (params (NewHolster :type "EHolster Enum" :default "EH_None"))
  ;[0.099 0.219 0.36 1 32] Игрок
  ;;[0.02604 0.02604 0.02604 1 24] Скрипты
  (`|PlayMontage` (`self.Mesh`) "/Game/TestTask/Blueprint/Animation/Rifleman/Misc/AS_Rifle_UnEquip_Montage.AS_Rifle_UnEquip_Montage"
    (:`OnCompleted`
      (`/Game/TestTask/Blueprint/Components/AC_WeaponComponent.SetGunSelect` (`self.Weapon Component`) NewHolster))))

(event `InputAction|SelectMain`
  (params (Key :type "Key Structure"))
  ;[0.099 0.219 0.36 1 32] Игрок
  ;;[0.02604 0.02604 0.02604 1 24] Скрипты
  (:`Pressed`
    (`self.ROS_SetGunSelect` "EH_Main")))

(event `InputAction|SelectSecond`
  (params (Key :type "Key Structure"))
  ;[0.099 0.219 0.36 1 32] Игрок
  ;;[0.02604 0.02604 0.02604 1 24] Скрипты
  (:`Pressed`
    (`self.ROS_SetGunSelect` "EH_Second")))

(event `InputAction|Aiming`
  (params (Key :type "Key Structure"))
  ;[0.099 0.219 0.36 1 32] Игрок
  ;;[0.02604 0.02604 0.02604 1 24] Скрипты
  (:`Pressed`
    (`self.SetAiming` true))
  (:`Released`
    (`self.SetAiming` false)))

(event `ROS_SetFire`
  (params (bEnabled :type Boolean))
  ;[0.099 0.219 0.36 1 32] Игрок
  ;;[0.02604 0.02604 0.02604 1 24] Скрипты
  (`self.MC_SetFire` bEnabled))

(event `MC_SetFire`
  (params (bEnabled :type Boolean))
  ;[0.099 0.219 0.36 1 32] Игрок
  ;;[0.02604 0.02604 0.02604 1 24] Скрипты
  (bind _gunptr (`self.OnActionGun`)
    (:`Valid`
      (`GunBase.SetFire` _gunptr bEnabled))))

(event `ROS_OnReload`
  ;[0.099 0.219 0.36 1 32] Игрок
  ;;[0.02604 0.02604 0.02604 1 24] Скрипты
  (`self.MC_OnReload`))

(event `MC_OnReload`
  ;[0.099 0.219 0.36 1 32] Игрок
  ;;[0.02604 0.02604 0.02604 1 24] Скрипты
  (bind _gunptr (`self.OnActionGun`)
    (:`Valid`
      (`GunBase.OnReload` _gunptr))))

(event `self.Weapon Component.OnGunAdd`
  (params (NewGun :type "/Game/TestTask/Blueprint/Weapon/BP_GunBase Object Reference"))
  ;[0.099 0.219 0.36 1 32] Игрок
  ;;[0.02604 0.02604 0.02604 1 24] Скрипты
  (`self.K2_AttachToComponent` NewGun (`self.Mesh`) (`.SocketAttach` (break `Gun` (`GunBase.Gun` NewGun))) "SnapToTarget" "SnapToTarget" "SnapToTarget" true))

(event `SetAiming`
  (params (bEnabled :type Boolean))
  ;[0.099 0.219 0.36 1 32] Игрок
  ;;[0.02604 0.02604 0.02604 1 24] Скрипты
  (`TimelineComponent.SetPlayRate` (`self.Aiming TM`) (/ 1.0 (`self.SpeedAimingMultiplay`)))
  (if bEnabled
    (bind (_direction _aim_alpha) (`Timeline|Aiming TM` :!label _label)
      (:`Update`
        (set `SpringArmComponent.TargetArmLength` (`KismetMathLibrary.Lerp` (`self.BaseArmLenght`) (`self.TargetArmLenght`) _aim_alpha) (`self.SpringArm`))
        (`CameraComponent.SetFieldOfView` (`self.Camera`) (`KismetMathLibrary.Lerp` (`self.FOV Base`) (`self.FOV When Aim`) _aim_alpha))))
    (else
      (goto _label :!via `Reverse`))))

(event `self.Weapon Component.OnGunFire`
  ;[0.099 0.219 0.36 1 32] Игрок
  ;;[0.02604 0.02604 0.02604 1 24] Скрипты
  (`|PlayMontage` (`self.Mesh`) "/Game/TestTask/Blueprint/Animation/Rifleman/Misc/AS_Rifle_Fire_Montage.AS_Rifle_Fire_Montage"))

(event `self.ReceiveBeginPlay`
  ;[0.099 0.219 0.36 1 32] Игрок
  ;;[0.1354 0.1354 0.1354] В начале отключаем управление игроком
  (`self.DisableInput` (`GameplayStatics.GetPlayerController` 0)))

(event `ROS_OnDead`
  (params (Actor :type "Actor Object Reference"))
  ;[0.099 0.219 0.36 1 32] Игрок
  ;;[0.1458 0.1458 0.1458] Гибель персонажа
  (`self.MC_OnDead` Actor))

(event `self.Health Component.OnDead`
  (params (Actor :type "Actor Object Reference"))
  ;[0.099 0.219 0.36 1 32] Игрок
  ;;[0.1458 0.1458 0.1458] Гибель персонажа
  (`self.DisableInput` (`GameplayStatics.GetPlayerController` 0))
  (`self.ROS_OnDead` Actor))

(event `MC_OnDead`
  (params (Actor :type "Actor Object Reference"))
  ;[0.099 0.219 0.36 1 32] Игрок
  ;;[0.1458 0.1458 0.1458] Гибель персонажа
  (`PrimitiveComponent.SetCollisionEnabled` (`self.Mesh`) "PhysicsOnly")
  (`PrimitiveComponent.SetCollisionEnabled` (`self.CapsuleComponent`) "NoCollision")
  (`PrimitiveComponent.SetSimulatePhysics` (`self.Mesh`) true))

(fn `GetSpeed`
  (returns (ReturnValue :type "Float (double-precision)"))
  (return (`KismetMathLibrary.VSize` (`self.GetVelocity`))))

(fn `UserConstructionScript`
  (set `self.BaseArmLenght` (`SpringArmComponent.TargetArmLength` (`self.SpringArm`)))
  (`CameraComponent.SetFieldOfView` (`self.Camera`) (`self.FOV Base`)))