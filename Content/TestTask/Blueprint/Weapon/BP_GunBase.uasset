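; Base gun Blueprint that sets its skeletal mesh from the Gun data via a blocking load in construction and fills its ammo on BeginPlay.
; It binds fire delegates so a timeline adds recoil pitch to the instigator's controller until firing ends or ammo runs out.
; Hits on BI_Human actors trigger blood at the impact point.
; The owner's AC_HealthComponent death delegate is bound to stop firing.
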(event `self.ReceiveBeginPlay`
  ;[0.005208 0.005208 0.068 1 32] GUN SYSTEM
  ;;[0.02604 0.02604 0.02604] Begin Play
  (`KismetSystemLibrary.Delay` 0.0)
  (`self.Reset Ammo`)
  (`self.GetPlayerControllerRef`)
  (`self.BindDelegates`))

(event `OnBeginGunFire`
  ;[0.005208 0.005208 0.068 1 32] GUN SYSTEM
  ;;[0.1406 0.1406 0.1406] Простая логика отдачи при стрельбе
  (bind (_direction _newtrack_0) (`Timeline|Recoil TM` :!via `PlayFromStart` :!label _label)
    (:`Update`
      (bind _playercontrollerref (`self.PlayerControllerRef`)
        (:`then`
          (if (`self.bFire`)
            (`PlayerController.AddPitchInput` _playercontrollerref (* _newtrack_0 -1.0))))
        (:`else`)))))

(event `OnEndGunFire`
  ;[0.005208 0.005208 0.068 1 32] GUN SYSTEM
  ;;[0.1406 0.1406 0.1406] Простая логика отдачи при стрельбе
  (`KismetSystemLibrary.Delay` 0.0 :!label _label_2)
  (goto _label :!via `Stop`))

(event `OnAmmoGunNull`
  ;[0.005208 0.005208 0.068 1 32] GUN SYSTEM
  ;;[0.1406 0.1406 0.1406] Простая логика отдачи при стрельбе
  (goto _label_2))

(event `Reset Ammo`
  (bind (_ammomaxinmag _ammocurrentinmag _ammototalmax) (break `Ammo` (`.Ammo` (break `Gun` (`self.Gun`)))))
  ;[0.005208 0.005208 0.068 1 32] GUN SYSTEM
  ;;[0.1458 0.1458 0.1458] Устанавливает патроны до максимальных значений, общих и в магазине
  (`self.SetAmmoTotal` _ammototalmax)
  (`self.SetAmmoCurrent` _ammomaxinmag))

(event `OnFireGunHitResult`
  (params (HitInfo :type "HitResult Structure"))
  (bind (_bblockinghit _binitialoverlap _time _distance _location _impactpoint _normal _impactnormal _physmat _hitactor) (`GameplayStatics.BreakHitResult` HitInfo))
  ;[0.005208 0.005208 0.068 1 32] GUN SYSTEM
  ;;[0.1354 0.1354 0.1354] Если попали в объект который содержит интерфейс "человека", спавним брызги крови на нем
  (if (`KismetSystemLibrary.DoesImplementInterface` _hitactor "/Game/TestTask/Blueprint/Interface/BI_Human.BI_Human_C")
    (message `/Game/TestTask/Blueprint/Interface/BI_Human.SpawnBlood` _hitactor _location)))

(fn `BindDelegates`
  (bind _returnvalue (`self.GetOwner`))
  (bind _returnvalue_2 (`self.GetComponentByClass` _returnvalue "/Game/TestTask/Blueprint/Components/AC_HealthComponent.AC_HealthComponent_C"))
  ;[0.2292 0.2292 0.2292] Бинд делегатов стрельбы
  (add `self.OnFireHitResult` (`|CreateDelegate` :!event `OnFireGunHitResult`))
  (add `self.OnBeginFire` (`|CreateDelegate` :!event `OnBeginGunFire`))
  (add `self.OnEndFire` (`|CreateDelegate` :!event `OnEndGunFire`))
  (add `self.OnAmmoNull` (`|CreateDelegate` :!event `OnAmmoGunNull`))
  ;[0.2656 0.2656 0.2656] Бинд делегата гибели владельца
  (`/Engine/EditorBlueprintResources/StandardMacros.IsValid` _returnvalue
    (:`Is Valid`
      (`/Engine/EditorBlueprintResources/StandardMacros.IsValid` _returnvalue_2
        (:`Is Valid`
          (add `/Game/TestTask/Blueprint/Components/AC_HealthComponent.OnDead` _returnvalue_2 (`|CreateDelegate` :!event `OnOwnerDead`)))))))

(fn `GetPlayerControllerRef`
  (bind _asplayer_controller (cast `PlayerController` (`self.GetInstigatorController`)))
  (set `self.PlayerControllerRef` _asplayer_controller))

(fn `OnOwnerDead`
  (params (Actor :type "Actor Object Reference"))
  (`self.OnStopFire`))

(fn `UserConstructionScript`
  ;[0.1406 0.1406 0.1406] Загружаем мешь
  (bind _returnvalue (`KismetSystemLibrary.LoadAsset_Blocking` (`.Mesh` (break `Gun` (`self.Gun`)))))
  (bind _asskeletal_mesh (cast `SkeletalMesh` _returnvalue))
  (`SkinnedMeshComponent.SetSkinnedAssetAndUpdate` (`self.GunMesh`) _asskeletal_mesh true))