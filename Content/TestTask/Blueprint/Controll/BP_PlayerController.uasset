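; BP_PlayerController is the player controller that handles the client side of a round's UI and input control.
; Its ROC-prefixed events, commented as the client part, create and add the round timer and end-round widgets to the viewport.
; Two more events enable or disable input on the controlled pawn, passing this controller.
; Nothing in this graph calls these events, and the construction script is empty.
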(event `ROC_ShowTimerRound`
  ;[0.4757 0.642 1 1 32] Клиентская часть
  ;;[0.1562 0.1562 0.1562] Спавнит виджет оставшиеся время раунда
  (bind _returnvalue (`|CreateWidget` "/Game/TestTask/Widget/HUD/WB_RoundTime.WB_RoundTime_C"))
  (`UserWidget.AddToViewport` _returnvalue 0))

(event `ROC_EnableInput`
  ;[0.4757 0.642 1 1 32] Клиентская часть
  ;;[0.1562 0.1562 0.1562] Включает управление игроку
  (`self.EnableInput` (`self.K2_GetPawn`) self))

(event `ROC_DisableInput`
  ;[0.4757 0.642 1 1 32] Клиентская часть
  ;;[0.1562 0.1562 0.1562] Отключает управление игроку
  (`self.DisableInput` (`self.K2_GetPawn`) self))

(event `ROC_ShowEndRound`
  ;[0.4757 0.642 1 1 32] Клиентская часть
  ;;[0.2292 0.2292 0.2292] Спавнит виджет конец раунда
  (bind _returnvalue (`|CreateWidget` "/Game/TestTask/Widget/HUD/WB_EndRound.WB_EndRound_C"))
  (`UserWidget.AddToViewport` _returnvalue 0))

(fn `UserConstructionScript`)