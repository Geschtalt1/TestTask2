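; AC_HealthComponent is a health component that extends a parent component managing an Ability amount and signals its owner's death.
; BindDelegates adds a binding to the owner's point-damage event after the parent's bindings, but the OnTakePointDamageOwner handler is empty.
; SetCurrentAmount runs the parent logic, then calls the OnDead dispatcher with the owner whenever the current amount is zero or below.
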(event `self.ReceiveBeginPlay`
  ;[0.1354 0.1354 0.1354] Отрабатывает родительскую логику
  (`parent.ReceiveBeginPlay`))

(event `OnTakePointDamageOwner`
  (params (DamagedActor :type "Actor Object Reference") (Damage :type "Float (single-precision)") (InstigatedBy :type "Controller Object Reference") (HitLocation :type "Vector Structure") (FHitComponent :type "PrimitiveComponent Object Reference") (BoneName :type Name) (ShotFromDirection :type "Vector Structure") (DamageType :type "DamageType Object Reference") (DamageCauser :type "Actor Object Reference")))

(fn `BindDelegates`
  (`parent.BindDelegates`)
  ;[0.1406 0.1406 0.1406] Привязываем делегат получения урона владельцем компонента
  (add `Actor.OnTakePointDamage` (`self.GetOwner`) (`|CreateDelegate` :!event `OnTakePointDamageOwner`)))

(fn `SetCurrentAmount`
  (params (NewCurrent :type "Float (double-precision)"))
  ;[0.1562 0.1562 0.1562] Проверяем если новое значение достигла нуля, вызываем делегат гибили владельца
  (`parent.SetCurrentAmount` NewCurrent)
  (if (<= (`.CurrentAmount_2_E2080C1243B590304AF94CB1A818C2D0` (break `/Game/TestTask/Blueprint/Struct/S_Ability` (`self.Ability`))) 0.0)
    (`self.OnDead` (`self.GetOwner`))))