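; Actor component that holds an ability as a current and maximum amount in an SAbility struct, like a resource pool.
; Setters clamp the current amount to the maximum, make the maximum non-negative and broadcast each change through event dispatchers.
; A zero-length delay after BeginPlay defers Init, which calls the empty BindDelegates hook and broadcasts starting values to outside subscribers.
; IsAbility reports whether any amount remains.
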(event `self.ReceiveBeginPlay`
  ;[0.1146 0.1146 0.1146] Инициализация компонента способности
  (`KismetSystemLibrary.Delay` 0.0)
  (`self.Init`))

(fn `BindDelegates`
  (return))

(fn `Init`
  (bind (_currentamount _maximumamount) (break `/Game/TestTask/Blueprint/Struct/S_Ability` (`self.Ability`)))
  ;[0.09375 0.09375 0.09375] Привязываем делегаты и рассылаем значения, если подписались из вне
  (`self.BindDelegates`)
  (`self.SetCurrentAmount` _currentamount)
  (`self.SetMaximumAmount` _maximumamount))

(fn `IsAbility`
  (returns (bReturnValue :type Boolean))
  (bind _ability_currentamount (break `/Game/TestTask/Blueprint/Struct/S_Ability` (`self.Ability`)))
  ;[0.1979 0.1979 0.1979] Возращает true, если кол-во текущей способности больше нуля
  (return (> _ability_currentamount 0.0)))

(fn `SetCurrentAmount`
  (params (NewCurrent :type "Float (double-precision)"))
  (bind (_currentamount _maximumamount) (break `/Game/TestTask/Blueprint/Struct/S_Ability` (`self.Ability`)))
  ;[0.125 0.125 0.125] Устанавливае текущее кол-во способности
  (setmembers `/Game/TestTask/Blueprint/Struct/S_Ability` :`StructRef` (`self.Ability`) :`CurrentAmount` (`KismetMathLibrary.FClamp` NewCurrent 0.0 _maximumamount))
  (`self.OnNewCurrentAmount` _currentamount))

(fn `SetMaximumAmount`
  (params (NewMax :type "Float (double-precision)"))
  ;[0.125 0.125 0.125] Устанавливаем максимальное кол-во способности
  (bind _structout (setmembers `/Game/TestTask/Blueprint/Struct/S_Ability` :`StructRef` (`self.Ability`) :`MaximumAmount` (`KismetMathLibrary.Abs` NewMax)))
  (`self.OnNewMaximumAmount` (`.MaximumAmount_4_F94BF97E494346B5C8E81EA551BCC0C4` (break `/Game/TestTask/Blueprint/Struct/S_Ability` _structout))))